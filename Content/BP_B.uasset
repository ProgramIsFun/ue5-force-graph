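; BP_B is an actor that moves its Sphere component in a straight line from BeginLocation toward EndLocation, then destroys itself.
; On BeginPlay, the Go event starts a fast looping timer that drives Move in place of Tick.
; Each Move offsets the Sphere by a fixed Speed step without sweeping, until it is within a small tolerance of EndLocation and the timer is cleared.
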(event Custom|Move
  (if (Utilities|Operators|EqualEqual (Transformation|GetWorldLocation (Variables|Default|GetSphere)) (Variables|Default|GetEndLocation) 1e+01)
    (Utilities|Time|ClearandInvalidateTimerbyHandle (Variables|Default|GetTimer))
    (Actor|DestroyActor)
    (else
      (Transformation|AddWorldOffset (Variables|Default|GetSphere) (* (Math|Vector|Normalize (- (Variables|Default|GetEndLocation) (Variables|Default|GetBeginLocation))) (Variables|Default|GetSpeed)) false false))))

(event Custom|Go
  (bind _returnvalue (Utilities|Time|SetTimerbyEvent (delegate Custom|Move) 0.02 true))
  (Variables|Default|SetTimer _returnvalue))

(event EventBeginPlay
  (CallFunction|Go))

(fn ConstructionScript)